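; BP_Ram is a grabbable RAM stick that snaps into a slot on a board actor (Placa) when released.
; When its GrabComponent fires OnDropped, it runs a small stationary sphere trace for physics bodies at the CorsairRGB component's "join" socket.
; If the hit actor is Placa, it attaches itself to socket "ram1", snapping location, rotation and scale, with debug prints along the way.
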(event OnDropped(GrabComponent)
  (bind _corsair_rgb (Variables|Default|GetCorsair_RGB))
  (bind _placa (Variables|Default|GetPlaca))
  (bind _returnvalue (Transformation|GetSocketLocation _corsair_rgb "join"))
  (Development|PrintString "Hello")
  (bind _outhit (Collision|SphereTraceForObjects _returnvalue _returnvalue 1e+01 (Utilities|Array|MakeArray "ObjectTypeQuery4") false 0 "None"))
  (if (== (.HitActor (Collision|BreakHitResult _outhit)) _placa)
    (Development|PrintString "FUNCIOAAAAAAAAAAAAAAAAAAAAAAAAAAAAAAAAAA")
    (Transformation|AttachActorToActor _placa "ram1" "SnapToTarget" "SnapToTarget" "SnapToTarget" false)))

(fn ConstructionScript)